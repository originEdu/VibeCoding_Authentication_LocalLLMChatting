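; Path actor for a tower-defense level that defines a fixed winding balloon route and renders it as a road.
; The construction script rebuilds the spline from hardcoded points, then adds a spline mesh cube per segment, scaled by RoadWidth and RoadThickness and bent along the spline tangents.
; GetPathLength and GetTransformAtDistance expose the spline length and world-space transform at a given distance.
; The event graph holds no active logic.
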(event EventBeginPlay)

(event Collision|EventActorBeginOverlap
  (params (OtherActor :type Actor%20Object%20Reference)))

(event EventTick
  (params (DeltaSeconds :type Float%20%28single-precision%29)))

(fn ConstructionScript
  (bind _returnvalue (Math|Float|MakeLiteralFloat 1e+02))
  (bind _returnvalue_2 (Math|Float|MakeLiteralFloat 1e+02))
  (bind _pathspline (Variables|Default|GetPathSpline))
  (bind _roadwidth (Variables|Default|GetRoadWidth))
  (bind _roadthickness (Variables|Default|GetRoadThickness))
  (bind _returnvalue_3 (Spline|GetNumberOfSplinePoints _pathspline))
  (bind _returnvalue_4 (/ _roadwidth _returnvalue))
  (bind _returnvalue_5 (/ _roadthickness _returnvalue_2))
  (bind _returnvalue_6 (Math|Vector2D|MakeVector2D _returnvalue_4 _returnvalue_5))
  (Spline|ClearSplinePoints _pathspline false)
  (Spline|AddSplinePoint _pathspline (Math|Vector|MakeVector -3.5e+03 -3e+03 2e+01) "Local" false)
  (Spline|AddSplinePoint _pathspline (Math|Vector|MakeVector -1e+03 -3e+03 2e+01) "Local" false)
  (Spline|AddSplinePoint _pathspline (Math|Vector|MakeVector 1.5e+03 -2e+03 2e+01) "Local" false)
  (Spline|AddSplinePoint _pathspline (Math|Vector|MakeVector 2.5e+03 0.0 2e+01) "Local" false)
  (Spline|AddSplinePoint _pathspline (Math|Vector|MakeVector 1e+03 1.5e+03 2e+01) "Local" false)
  (Spline|AddSplinePoint _pathspline (Math|Vector|MakeVector -1.5e+03 1e+03 2e+01) "Local" false)
  (Spline|AddSplinePoint _pathspline (Math|Vector|MakeVector -2.5e+03 2.5e+03 2e+01) "Local" false)
  (Spline|AddSplinePoint _pathspline (Math|Vector|MakeVector 0.0 3.2e+03 2e+01) "Local" false)
  (Spline|AddSplinePoint _pathspline (Math|Vector|MakeVector 3.5e+03 3e+03 2e+01) "Local" true)
  (if (>= _returnvalue_3 (Class|KismetSystemLibrary|MakeLiteralInteger 2))
    (for _index (range 0 (- (- _returnvalue_3 (Class|KismetSystemLibrary|MakeLiteralInteger 1)) (Class|KismetSystemLibrary|MakeLiteralInteger 1)))
      (bind _returnvalue_7 (AddComponent|AddSplineMeshComponent self false (Math|Transform|MakeTransform "0, 0, 0")))
      (Components|StaticMesh|SetStaticMesh _returnvalue_7 "/Engine/BasicShapes/Cube.Cube")
      (SplineMesh|SetForwardAxis _returnvalue_7 "X" false)
      (SplineMesh|SetStartScale _returnvalue_7 _returnvalue_6 false :!class /Script/Engine.SplineMeshComponent)
      (SplineMesh|SetEndScale _returnvalue_7 _returnvalue_6 false :!class /Script/Engine.SplineMeshComponent)
      (SplineMesh|SetStartandEnd _returnvalue_7 (Spline|GetLocationatSplinePoint _pathspline _index "Local") (Spline|GetTangentatSplinePoint _pathspline _index "Local") (Spline|GetLocationatSplinePoint _pathspline (+ _index (Class|KismetSystemLibrary|MakeLiteralInteger 1)) "Local") (Spline|GetTangentatSplinePoint _pathspline (+ _index (Class|KismetSystemLibrary|MakeLiteralInteger 1)) "Local") true :!class /Script/Engine.SplineMeshComponent))))

(fn GetPathLength
  (return (Spline|GetSplineLength (Variables|Default|GetPathSpline))))

(fn GetTransformatDistance
  (params (Distance :type Float%20%28double-precision%29))
  (return (Spline|GetTransformatDistanceAlongSpline (Variables|Default|GetPathSpline) Distance "World" false)))
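; BP_BalloonSpawner spawns balloons at regular intervals at the start of a path in a TD game.
; On BeginPlay it starts a looping timer at SpawnInterval, or prints a warning and stays disabled if no Path is set.
; Each timer call spawns a BP_Balloon at the path's zero-point transform, ignoring collision, and passes it the Path reference.
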(event EventBeginPlay
  (Utilities|IsValid (Variables|Default|GetPath)
    (:Is%20Valid
      (Utilities|Time|SetTimerbyFunctionName self "SpawnBalloon" (Variables|Default|GetSpawnInterval) true))
    (:Is%20Not%20Valid
      (Development|PrintString "BP_BalloonSpawner: Path is not set - spawner disabled"))))

(event Collision|EventActorBeginOverlap
  (params (OtherActor :type Actor%20Object%20Reference)))

(event EventTick
  (params (DeltaSeconds :type Float%20%28single-precision%29)))

(fn ConstructionScript)

(fn SpawnBalloon
  (bind _returnvalue (Default|PathTransformat (Variables|Default|GetPath) 0.0))
  (bind _returnvalue_2 (Game|SpawnActorfromClass "/Game/TD/BP_Balloon.BP_Balloon_C" _returnvalue "AlwaysSpawn" "MultiplyWithRoot" 0 0))
  (Variables|/Game/TD/BP_Balloon.BP_Balloon_C|SetPath _returnvalue_2 (Variables|Default|GetPath)))
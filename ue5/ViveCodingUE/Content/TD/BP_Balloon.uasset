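; BP_Balloon is an actor, in what appears to be a tower defense game, that travels along an assigned Path and destroys itself at the end.
; BeginPlay prints an error and destroys the balloon if Path is unset.
; Tick advances distance by Speed and delta time, then teleports the balloon to the location and rotation the Path returns.
; An unreachable copy of the movement logic calls differently named Path functions.
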(event EventBeginPlay
  (Utilities|IsValid (Variables|Default|GetPath)
    (:Is%20Not%20Valid
      (Development|PrintString "BP_Balloon: Path is not set - destroying")
      (Actor|DestroyActor self))))

(event Collision|EventActorBeginOverlap
  (params (OtherActor :type Actor%20Object%20Reference)))

(event EventTick
  (params (DeltaSeconds :type Float%20%28single-precision%29))
  (bind _self self)
  (bind _path (Variables|Default|GetPath))
  (Utilities|IsValid _path
    (:Is%20Valid
      (Variables|Default|SetDistanceAlongPath (+ (Variables|Default|GetDistanceAlongPath) (* (Variables|Default|GetSpeed) DeltaSeconds)))
      (bind _returnvalue (Default|PathTotalLength _path))
      (if (>= (+ (Variables|Default|GetDistanceAlongPath) (* (Variables|Default|GetSpeed) DeltaSeconds)) _returnvalue)
        (Actor|DestroyActor _self)
        (else
          (bind _returnvalue_2 (Default|PathTransformat _path (+ (Variables|Default|GetDistanceAlongPath) (* (Variables|Default|GetSpeed) DeltaSeconds))))
          (Transformation|SetActorLocationAndRotation _self (.Location (Math|Transform|BreakTransform _returnvalue_2)) (.Rotation (Math|Transform|BreakTransform _returnvalue_2)) false true))))))

(fn ConstructionScript)